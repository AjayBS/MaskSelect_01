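; Player character that moves in discrete steps when a mapped direction key is pressed.
; Key presses look up a step vector in DirectionKeys, and a timeline lerps the actor to the offset location without sweep.
; Each finished step spends a MovePoint if any remain and repeats while the key stays held.
; MovePoints are only checked after a step, so a fresh press still moves at zero.
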(event `Key|AnyKey`
  (params (Key :type "Key Structure"))
  (bind _returnvalue (> (`self.MovePoints`) 0))
  (bind (_value _returnvalue_2) (`BlueprintMapLibrary.Map_Find` (`self.DirectionKeys`) Key))
  (:`Pressed`
    (set `self.ShouldTakeAStep` true)
    (if (and _returnvalue_2 (not (`TimelineComponent.IsPlaying` (`self.Timeline_0`))) (`self.ShouldTakeAStep`))
      (bind _output_get (set `self.DirectionStepSize` _value))
      (bind _output_get_2 (set `self.StartLoc` (`self.K2_GetActorLocation`) :!label _label))
      (set `self.EndLoc` (+ _output_get_2 _output_get))
      (bind (_direction _movealpha) (`Timeline|Timeline_0` :!via `PlayFromStart`)
        (:`Update`
          (`self.K2_SetActorLocation` (`KismetMathLibrary.VLerp` (`self.StartLoc`) (`self.EndLoc`) _movealpha)))
        (:`Finished`
          (if _returnvalue
            (`/Engine/EditorBlueprintResources/StandardMacros.DecrementInt` (`self.MovePoints`)
              (:`  `
                (if (`self.ShouldTakeAStep`)
                  (`self.TakeNextStep`))))
            (else
              (set `self.ShouldTakeAStep` _returnvalue)))))))
  (:`Released`
    (set `self.ShouldTakeAStep` false)))

(event `TakeNextStep`
  (goto _label))

(fn `UserConstructionScript`)