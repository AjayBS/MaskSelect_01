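; Coin mesh component representing a color-typed collectible that can be activated, deactivated and completed.
; Assigning a color stores its type and applies the matching material to the mesh.
; Activation only succeeds when the passed color matches the stored type, swapping to an active material, while deactivation swaps to another material and clears the active flag.
; Completion is only recorded while the coin is active.
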(fn `SetActiveStatus`
  (params (Color :type "/Game/Essentials/E_TileColorType Enum" :default "NewEnumerator1"))
  (if (`|EnumEquality` Color (`self.ColorType`))
    (`self.SetMaterial` 0 "/Engine/MapTemplates/Materials/BasicAsset03.BasicAsset03")
    (set `self.bIsCollectibleActive` true)))

(fn `SetColorTypeAndMaterial`
  (params (Color :type "/Game/Essentials/E_TileColorType Enum" :default "NewEnumerator1"))
  (bind _output_get (set `self.ColorType` Color))
  (`/Game/Essentials/BFL_CommonFUnctions.SetMaterialAccordingtoColor` self _output_get))

(fn `SetComplete`
  (if (`self.bIsCollectibleActive`)
    (set `self.bCompleted` true)))

(fn `SetDeactive`
  (`self.SetMaterial` 0 "/Engine/MapTemplates/Materials/BasicAsset01.BasicAsset01")
  (set `self.bIsCollectibleActive` false))